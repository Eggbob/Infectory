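; BP_Door_A is an automatic sliding door that opens on trigger overlap, optionally requiring an inventory item.
; When NeedItem is set, CheckItem queries the overlapping actor's inventory through IFCharacterPlayer for NeedItemID.
; Opening plays sound and steam effects while a Timeline lerps the door mesh between closed and open positions.
; On Timeline finish it changes an optional scanner's screen material and, after opening, closes by reversing the Timeline following a short delay.
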(event OnComponentBeginOverlap(Trigger)
  (params (OverlappedComponent :type Primitive%20Component%20Object%20Reference) (OtherActor :type Actor%20Object%20Reference) (OtherComp :type Primitive%20Component%20Object%20Reference) (OtherBodyIndex :type Integer) (bFromSweep :type Boolean) (SweepResult :type Hit%20Result%20Structure%20%28by%20ref%29))
  (bind _scanner (Variables|Default|GetScanner))
  (if (Variables|Default|GetbNeedItem)
    (bind _newparam (CallFunction|CheckItem OtherActor))
    (if _newparam
      (if (not (Variables|Default|GetbIsOpen)) :!label _label
        (Variables|Default|SetbIsOpen true)
        (Audio|PlaySoundatLocation "/Game/Assets/Map/sound/Door_open.Door_open" (Transformation|GetActorLocation) "0, 0, 0" 1.0 1.0 0.0 0 0 0 0)
        (Components|Activation|Activate (Variables|Default|GetSteamDoor2) false)
        (Variables|Default|SetbToReverse true)
        (bind _doorposition (Timeline|Timeline_0 Play)
          (:Update
            (Transformation|SetRelativeLocation (Variables|Default|GetDoor_Small_A) (Math|Vector|Lerp(Vector) (Variables|Door|GetDoorClosed) (Variables|Door|GetDoorOpen) _doorposition) false false))
          (:Finished
            (if (Utilities|IsValid _scanner)
              (Rendering|Material|SetMaterial (Actor|GetComponentbyClass _scanner "/Script/Engine.StaticMeshComponent") 1 "/Game/StarterBundle/ModularScifiProps/Materials/MI_HandScanner_Screen2.MI_HandScanner_Screen2"))
            (if (Variables|Default|GetbToReverse)
              (Utilities|FlowControl|Delay 1.5)
              (CallFunction|CloseDoor))))))
    (else
      (goto _label))))

(event Custom|CloseDoor
  (bind _scanner (Variables|Default|GetScanner))
  (Variables|Default|SetbToReverse false)
  (Audio|PlaySoundatLocation "/Game/Assets/Map/sound/Door_open.Door_open" (Transformation|GetActorLocation) "0, 0, 0" 1.0 1.0 0.0 0 0 0 0)
  (Variables|Default|SetbIsOpen false)
  (bind _doorposition (Timeline|Timeline_0 ReverseFromEnd)
    (:Update
      (Transformation|SetRelativeLocation (Variables|Default|GetDoor_Small_A) (Math|Vector|Lerp(Vector) (Variables|Door|GetDoorClosed) (Variables|Door|GetDoorOpen) _doorposition) false false))
    (:Finished
      (if (Utilities|IsValid _scanner)
        (Rendering|Material|SetMaterial (Actor|GetComponentbyClass _scanner "/Script/Engine.StaticMeshComponent") 1 "/Game/StarterBundle/ModularScifiProps/Materials/MI_HandScanner_Screen2.MI_HandScanner_Screen2"))
      (if (Variables|Default|GetbToReverse)
        (Utilities|FlowControl|Delay 1.5)
        (CallFunction|CloseDoor)))))

(fn ConstructionScript)

(fn CheckItem
  (params (Actor :type Actor%20Object%20Reference))
  (bind _asifcharacter_player (Utilities|Casting|CastToIFCharacterPlayer Actor))
  (bind _returnvalue (Class|IFCharacterPlayer|GetInventory _asifcharacter_player))
  (bind _returnvalue_2 (Class|IFInventory|CheckItem _returnvalue (Variables|Default|GetNeedItemID)))
  (return _returnvalue_2))