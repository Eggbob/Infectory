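; BP_Tumor is a tumor actor that can be switched on and off and is permanently disabled after its second deactivation.
; Activation refills its HP, enables query-only sphere collision and turns on the material Glow parameter.
; Deactivation reverses the glow and collision and increments a destroy counter; at two, it sets the Active material parameter and clears CanActive.
; Damage handling and the triggers for both events are not in this graph.
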(event EventActiveTumor
  (Collision|SetCollisionEnabled (Variables|Default|GetSphereComp) "QueryOnly")
  (Variables|Default|SetTumorCurHP (Variables|Default|GetTumorHP))
  (Variables|Default|SetbIsActivate true)
  (Variables|Default|SetGlowParam 1.0)
  (Rendering|Material|SetScalarParameterValueonMaterials (Variables|Default|GetSkeletalMeshComp) "Glow" (Variables|Default|GetGlowParam)))

(event EventDeActiveTumor
  (Math|Integer|IncrementInt (Variables|Default|GetDestroyCount)
    (:%20%20
      (Variables|Default|SetbIsActivate false)
      (Variables|Default|SetGlowParam 0.0)
      (Rendering|Material|SetScalarParameterValueonMaterials (Variables|Default|GetSkeletalMeshComp) "Glow" (Variables|Default|GetGlowParam))
      (Collision|SetCollisionEnabled (Variables|Default|GetSphereComp) "NoCollision")
      (if (== (Variables|Default|GetDestroyCount) 2)
        (Rendering|Material|SetScalarParameterValueonMaterials (Variables|Default|GetSkeletalMeshComp) "Active" 1.0)
        (Variables|Default|SetbCanActive false)))))

(fn ConstructionScript)