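; IF_KeyItemBox is an interactable box that gives the player a key item when opened.
; Overlapping its trigger enables input and caches the IFCharacterPlayer, and pressing T runs the opening once.
; LaunchBox hides the prompt text, spawns two steam vent emitters and raises the lid along a timeline.
; When the timeline finishes, it stops the steam, adds ItemData to the inventory and updates the player's notification text.
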(event OnComponentBeginOverlap(Box)
  (params (OverlappedComponent :type Primitive%20Component%20Object%20Reference) (OtherActor :type Actor%20Object%20Reference) (OtherComp :type Primitive%20Component%20Object%20Reference) (OtherBodyIndex :type Integer) (bFromSweep :type Boolean) (SweepResult :type Hit%20Result%20Structure%20%28by%20ref%29))
  (Input|EnableInput (Game|GetPlayerController 0))
  (bind _asifcharacter_player (Utilities|Casting|CastToIFCharacterPlayer OtherActor))
  (Variables|Default|SetAs%20IFCharacter%20Player _asifcharacter_player))

(event OnComponentEndOverlap(Box)
  (params (OverlappedComponent :type Primitive%20Component%20Object%20Reference) (OtherActor :type Actor%20Object%20Reference) (OtherComp :type Primitive%20Component%20Object%20Reference) (OtherBodyIndex :type Integer))
  (Input|DisableInput (Game|GetPlayerController 0)))

(event Custom|LaunchBox
  (Rendering|SetVisibility (Variables|Default|GetTextRender) false false)
  (bind _returnvalue (Effects|SpawnEmitteratLocation "/Game/InfinityBladeEffects/Effects/FX_Ambient/Steam/P_VentSteam.P_VentSteam" (Transformation|GetWorldLocation (Variables|Default|GetBillboard))))
  (Variables|Default|SetSteamParticle1 _returnvalue)
  (bind _returnvalue_2 (Effects|SpawnEmitteratLocation "/Game/InfinityBladeEffects/Effects/FX_Ambient/Steam/P_VentSteam_Fast.P_VentSteam_Fast" (Transformation|GetWorldLocation (Variables|Default|GetBillboard1))))
  (Variables|Default|SetSteamParticle2 _returnvalue_2)
  (bind _newtrack_0 (Timeline|BoxOpenTimeline Play)
    (:Update
      (Transformation|SetRelativeLocation (Variables|Default|GetBoxTopMesh) (Math|Vector|Lerp(Vector) (Variables|Default|GetCloseVector) (Variables|Default|GetUpVector) _newtrack_0) false false))
    (:Finished
      (Components|Activation|Deactivate (Variables|Default|GetSteamParticle1))
      (Components|Activation|Deactivate (Variables|Default|GetSteamParticle2))
      (bind _returnvalue_3 (Class|IFCharacterPlayer|GetInventory (Variables|Default|GetAs%20IFCharacter%20Player)))
      (Class|IFInventory|AddItem _returnvalue_3 (Variables|Default|GetItemData))
      (bind _returnvalue_4 (Class|IFCharacterPlayer|GetUserWidget (Variables|Default|GetAs%20IFCharacter%20Player)))
      (Class|IFUserWidget|UpdateNotifyText _returnvalue_4 (Variables|Default|GetNotifyText)))))

(event Input|KeyboardEvents|T
  (params (Key :type Key%20Structure :default "None"))
  (:Pressed
    (if (not (Variables|Default|GetbIsPress))
      (Variables|Default|SetbIsPress true)
      (CallFunction|LaunchBox))))

(fn ConstructionScript)