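; BP_TurretOpen is an interactable that activates a set of turrets when the player holds F near it.
; Box overlap enables and disables player input on the actor, without checking which actor overlaps.
; While F is held, Tick fills a progress bar from the widget component, and releasing F calls FinishPercent on it.
; A full bar calls PerformTurret on every entry in Turrets, latched by IsStart to fire once.
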(event OnComponentBeginOverlap(Box)
  (params (OverlappedComponent :type Primitive%20Component%20Object%20Reference) (OtherActor :type Actor%20Object%20Reference) (OtherComp :type Primitive%20Component%20Object%20Reference) (OtherBodyIndex :type Integer) (bFromSweep :type Boolean) (SweepResult :type Hit%20Result%20Structure%20%28by%20ref%29))
  (Input|EnableInput (Game|GetPlayerController 0)))

(event OnComponentEndOverlap(Box)
  (params (OverlappedComponent :type Primitive%20Component%20Object%20Reference) (OtherActor :type Actor%20Object%20Reference) (OtherComp :type Primitive%20Component%20Object%20Reference) (OtherBodyIndex :type Integer))
  (Input|DisableInput (Game|GetPlayerController 0)))

(event Custom|LaunchTurret
  (for _array_element (Variables|Default|GetTurrets)
    (Class|IFFieldTurret|PerformTurret _array_element)))

(event EventTick
  (params (DeltaSeconds :type Float%20%28single-precision%29))
  (if (and (Variables|Default|GetbIsPress) (<= (Variables|/Game/Assets/UI/BP_ProgressBar.BP_ProgressBar_C|GetPerecent (Variables|Default|GetProgressBar)) 1.0))
    (Default|UpdatePercent (Variables|Default|GetProgressBar))
    (elif (and (>= (Variables|/Game/Assets/UI/BP_ProgressBar.BP_ProgressBar_C|GetPerecent (Variables|Default|GetProgressBar)) 1.0) (not (Variables|Default|GetbIsStart)))
      (Variables|Default|SetbIsStart true)
      (CallFunction|LaunchTurret))))

(event EventBeginPlay
  (bind _asbp_progress_bar (Utilities|Casting|CastToBP_ProgressBar (UserInterface|GetWidget (Variables|Default|GetProgressBarWidget))))
  (Variables|Default|SetProgressBar _asbp_progress_bar))

(event Input|KeyboardEvents|F
  (params (Key :type Key%20Structure :default "None"))
  (:Pressed
    (Variables|Default|SetbIsPress true))
  (:Released
    (Variables|Default|SetbIsPress false)
    (Default|FinishPercent (Variables|Default|GetProgressBar))))

(fn ConstructionScript)