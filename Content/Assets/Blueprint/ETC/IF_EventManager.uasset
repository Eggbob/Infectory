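; Interactable event manager actor that launches a one-time alarm event when the player holds F inside its trigger box.
; Holding F fills a progress-bar widget on Tick, and completion turns spotlights red, activates a turret, destroys a target actor with a particle effect and calls a timer.
; StartFlash toggles spotlight intensity, while FinishEvent restores white lighting and adds an item to the player's inventory.
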(event OnComponentBeginOverlap(Box)
  (params (OverlappedComponent :type Primitive%20Component%20Object%20Reference) (OtherActor :type Actor%20Object%20Reference) (OtherComp :type Primitive%20Component%20Object%20Reference) (OtherBodyIndex :type Integer) (bFromSweep :type Boolean) (SweepResult :type Hit%20Result%20Structure%20%28by%20ref%29))
  (Input|EnableInput (Game|GetPlayerController 0))
  (bind _asbp_player_character (Utilities|Casting|CastToBP_PlayerCharacter OtherActor))
  (Variables|Default|SetTargetActor _asbp_player_character))

(event OnComponentEndOverlap(Box)
  (params (OverlappedComponent :type Primitive%20Component%20Object%20Reference) (OtherActor :type Actor%20Object%20Reference) (OtherComp :type Primitive%20Component%20Object%20Reference) (OtherBodyIndex :type Integer))
  (Input|DisableInput (Game|GetPlayerController 0)))

(event Custom|StartEvent
  (if (not (Variables|Default|GetbIsStart))
    (CallFunction|EventAction)
    (Class|IFEventManager|StartTimer)))

(event EventStartFlash
  (bind _spotlights (Variables|Default|GetSpotLights))
  (if (Variables|Default|GetbIsLightOn)
    (for _array_element _spotlights
      (Rendering|Components|Light|SetIntensity (Variables|/Script/Engine.Light|GetLightComponent _array_element) 0.0))
    (Variables|Default|SetbIsLightOn false)
    (else
      (for _array_element_2 _spotlights
        (Rendering|Components|Light|SetIntensity (Variables|/Script/Engine.Light|GetLightComponent _array_element_2) (Variables|Default|GetMaxIntensity)))
      (Variables|Default|SetbIsLightOn true))))

(event EventFinishEvent
  (bind _returnvalue (Class|IFCharacterPlayer|GetInventory (Variables|Default|GetTargetActor)))
  (Class|IFInventory|AddItem _returnvalue (Variables|Default|GetItemData))
  (for _array_element (Variables|Default|GetSpotLights)
    (Rendering|Components|Light|SetIntensity (Variables|/Script/Engine.Light|GetLightComponent _array_element) (Variables|Default|GetMaxIntensity))
    (Rendering|Components|Light|SetLightColor (Variables|/Script/Engine.Light|GetLightComponent _array_element) "(R=1.000000,G=1.000000,B=1.000000,A=1.000000)" true)))

(event EventTick
  (params (DeltaSeconds :type Float%20%28single-precision%29))
  (bind _progressbar (Variables|Default|GetProgressBar))
  (bind _perecent (Variables|/Game/Assets/UI/BP_ProgressBar.BP_ProgressBar_C|GetPerecent _progressbar))
  (bind _returnvalue (<= _perecent 1.0))
  (if (and (Variables|Default|GetbIsPress) _returnvalue)
    (Default|UpdatePercent (Variables|Default|GetProgressBar))
    (elif (not (and _returnvalue (not (Variables|Default|GetbIsStart))))
      (CallFunction|StartEvent)
      (Variables|Default|SetbIsStart true))))

(event EventBeginPlay
  (bind _asbp_progress_bar (Utilities|Casting|CastToBP_ProgressBar (UserInterface|GetWidget (Variables|Default|GetProgressBarWidget))))
  (Variables|Default|SetProgressBar _asbp_progress_bar))

(event Input|KeyboardEvents|F
  (params (Key :type Key%20Structure :default "None"))
  (:Pressed
    (Variables|Default|SetbIsPress true))
  (:Released
    (Variables|Default|SetbIsPress false)
    (Default|FinishPercent (Variables|Default|GetProgressBar))))

(fn ConstructionScript)

(fn EventAction
  (bind _destroyactor (Variables|Default|GetDestroyActor))
  (for _array_element (Variables|Default|GetSpotLights)
    (Rendering|Components|Light|SetLightColor (Variables|/Script/Engine.Light|GetLightComponent _array_element) "(R=1.000000,G=0.000000,B=0.000000,A=1.000000)" true))
  (Class|IFFieldTurret|PerformTurret (Variables|Default|GetTurret))
  (Development|SetHiddeninGame (Variables|Default|GetProgressBarWidget) true false)
  (Effects|SpawnEmitteratLocation "/Game/Realistic_Starter_VFX_Pack_Vol2/Particles/Explosion/P_Molotov.P_Molotov" (Transformation|GetActorLocation _destroyactor))
  (Actor|DestroyActor _destroyactor)
  (AddComponent|AddAudioComponent false))