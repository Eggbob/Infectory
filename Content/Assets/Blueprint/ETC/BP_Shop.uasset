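; BP_Shop is an in-world shop actor that a player character uses through a trigger box.
; Entering the box enables the actor's input and binds the player's inventory to the shop widget; leaving disables input and ends shop mode.
; F swaps the pop-up prompt for the shop display and sets shop mode on the player.
; Other keys forward item selection, widget switching, Enter and Tab actions to the shop widget.
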(event OnComponentBeginOverlap(Box)
  (params (OverlappedComponent :type Primitive%20Component%20Object%20Reference) (OtherActor :type Actor%20Object%20Reference) (OtherComp :type Primitive%20Component%20Object%20Reference) (OtherBodyIndex :type Integer) (bFromSweep :type Boolean) (SweepResult :type Hit%20Result%20Structure%20%28by%20ref%29))
  (Input|EnableInput (Game|GetPlayerController 0))
  (bind _asbp_player_character (Utilities|Casting|CastToBP_PlayerCharacter OtherActor))
  (bind _output_get (Variables|Default|SetBPPlayerCharacter _asbp_player_character))
  (bind _returnvalue (Class|IFCharacterPlayer|GetInventory _output_get))
  (Class|IFShopWidget|BindInventory (Variables|Default|GetShopWidget) _returnvalue))

(event OnComponentEndOverlap(Box)
  (params (OverlappedComponent :type Primitive%20Component%20Object%20Reference) (OtherActor :type Actor%20Object%20Reference) (OtherComp :type Primitive%20Component%20Object%20Reference) (OtherBodyIndex :type Integer))
  (Input|DisableInput (Game|GetPlayerController 0))
  (Development|SetHiddeninGame (Variables|Default|GetPopUpWidget) false false)
  (Rendering|SetVisibility (Variables|Default|GetShopPopUpWidget) false false)
  (Class|IFCharacterPlayer|SetShopMode (Variables|Default|GetBPPlayerCharacter) false))

(event Input|KeyboardEvents|F
  (params (Key :type Key%20Structure :default "None"))
  (:Pressed
    (Development|SetHiddeninGame (Variables|Default|GetPopUpWidget) true false)
    (Class|IFShop|OpenShopWidget)
    (Rendering|SetVisibility (Variables|Default|GetShopPopUpWidget) true false)
    (Class|IFCharacterPlayer|SetShopMode (Variables|Default|GetBPPlayerCharacter) true)))

(event Input|KeyboardEvents|Left
  (params (Key :type Key%20Structure :default "None"))
  (:Pressed
    (Variables|Default|SetDirectionVector "(X=0.000000,Y=-1.000000)")
    (Class|IFShopWidget|SelectItem (Variables|Default|GetShopWidget) (Variables|Default|GetDirectionVector))))

(event Input|KeyboardEvents|Right
  (params (Key :type Key%20Structure :default "None"))
  (:Pressed
    (Variables|Default|SetDirectionVector "(X=0.000000,Y=1.000000)")
    (Class|IFShopWidget|SelectItem (Variables|Default|GetShopWidget) (Variables|Default|GetDirectionVector))))

(event Input|KeyboardEvents|Up
  (params (Key :type Key%20Structure :default "None"))
  (:Pressed
    (Variables|Default|SetDirectionVector "(X=1.000000,Y=0.000000)")
    (Class|IFShopWidget|SelectItem (Variables|Default|GetShopWidget) (Variables|Default|GetDirectionVector))))

(event Input|KeyboardEvents|Down
  (params (Key :type Key%20Structure :default "None"))
  (:Pressed
    (Variables|Default|SetDirectionVector "(X=-1.000000,Y=0.000000)")
    (Class|IFShopWidget|SelectItem (Variables|Default|GetShopWidget) (Variables|Default|GetDirectionVector))))

(event Input|KeyboardEvents|Q
  (params (Key :type Key%20Structure :default "None"))
  (:Pressed
    (Class|IFShopWidget|OpenWidget (Variables|Default|GetShopWidget) true)))

(event Input|KeyboardEvents|E
  (params (Key :type Key%20Structure :default "None"))
  (:Pressed
    (Class|IFShopWidget|OpenWidget (Variables|Default|GetShopWidget) false)))

(event Input|KeyboardEvents|Enter
  (params (Key :type Key%20Structure :default "None"))
  (:Pressed
    (Class|IFShopWidget|PerformEnterAction (Variables|Default|GetShopWidget))))

(event Input|KeyboardEvents|Tab
  (params (Key :type Key%20Structure :default "None"))
  (:Pressed
    (Class|IFShopWidget|PerformTabAction (Variables|Default|GetShopWidget))))

(fn ConstructionScript)