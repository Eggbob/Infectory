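; BP_ItemBox is an item container that gives its ItemData to the player's inventory when E is pressed nearby.
; Box overlap enables input for player 0, shows a prompt widget and calls OpenItemBox until the item is taken.
; E casts the overlapping actor to BP_PlayerCharacter, adds the item, sets IsGetItem and hides the widget.
; IsGetItem gates only the overlap, and input stays enabled until overlap ends.
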(event OnComponentBeginOverlap(Box)
  (params (OverlappedComponent :type Primitive%20Component%20Object%20Reference) (OtherActor :type Actor%20Object%20Reference) (OtherComp :type Primitive%20Component%20Object%20Reference) (OtherBodyIndex :type Integer) (bFromSweep :type Boolean) (SweepResult :type Hit%20Result%20Structure%20%28by%20ref%29))
  (if (not (Variables|Default|GetbIsGetItem))
    (Input|EnableInput (Game|GetPlayerController 0))
    (Rendering|SetVisibility (Variables|Default|GetWidget) true false)
    (Class|IFItemDropBox|OpenItemBox)))

(event OnComponentEndOverlap(Box)
  (params (OverlappedComponent :type Primitive%20Component%20Object%20Reference) (OtherActor :type Actor%20Object%20Reference) (OtherComp :type Primitive%20Component%20Object%20Reference) (OtherBodyIndex :type Integer))
  (Input|DisableInput (Game|GetPlayerController 0))
  (Rendering|SetVisibility (Variables|Default|GetWidget) false false))

(event Input|KeyboardEvents|E
  (params (Key :type Key%20Structure :default "None"))
  (:Pressed
    (bind _asbp_player_character (Utilities|Casting|CastToBP_PlayerCharacter (stale OnComponentBeginOverlap(Box) OtherActor)))
    (bind _returnvalue (Class|IFCharacterPlayer|GetInventory _asbp_player_character))
    (Class|IFInventory|AddItem _returnvalue (Variables|Default|GetItemData))
    (Variables|Default|SetbIsGetItem true)
    (Rendering|SetVisibility (Variables|Default|GetWidget) false false)))

(fn ConstructionScript)