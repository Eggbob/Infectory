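; BP_Turret is a turret actor that the player can recall when nearby.
; Box overlap toggles input for player 0 and a text prompt, without filtering the overlapping actor, and F calls RecallTurret on the owner's player character.
; While IsStart is set, Tick rotates the text toward the owner's pawn.
; When projectile movement stops, its updated component is reassigned to the capsule.
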(event OnProjectileStop(ProjectileMovement)
  (params (ImpactResult :type Hit%20Result%20Structure%20%28by%20ref%29))
  (Components|Movement|SetUpdatedComponent (Variables|Default|GetProjectileMovement) (Variables|Default|GetCapsuleComp)))

(event OnComponentBeginOverlap(Box)
  (params (OverlappedComponent :type Primitive%20Component%20Object%20Reference) (OtherActor :type Actor%20Object%20Reference) (OtherComp :type Primitive%20Component%20Object%20Reference) (OtherBodyIndex :type Integer) (bFromSweep :type Boolean) (SweepResult :type Hit%20Result%20Structure%20%28by%20ref%29))
  (Input|EnableInput (Game|GetPlayerController 0))
  (Development|SetHiddeninGame (Variables|Default|GetTextRender) false false))

(event OnComponentEndOverlap(Box)
  (params (OverlappedComponent :type Primitive%20Component%20Object%20Reference) (OtherActor :type Actor%20Object%20Reference) (OtherComp :type Primitive%20Component%20Object%20Reference) (OtherBodyIndex :type Integer))
  (Input|DisableInput (Game|GetPlayerController 0))
  (Development|SetHiddeninGame (Variables|Default|GetTextRender) true false))

(event EventTick
  (params (DeltaSeconds :type Float%20%28single-precision%29))
  (bind _textrender (Variables|Default|GetTextRender))
  (if (Variables|Default|GetbIsStart)
    (Transformation|SetWorldRotation _textrender (Math|Rotator|FindLookatRotation (Transformation|GetWorldLocation _textrender) (Transformation|GetActorLocation (Pawn|GetControlledPawn (Variables|Default|GetOwnerController)))) false false)))

(event EventBeginPlay
  (Development|SetHiddeninGame (Variables|Default|GetTextRender) true false))

(event Input|KeyboardEvents|F
  (params (Key :type Key%20Structure :default "None"))
  (:Pressed
    (bind _asbp_player_character (Utilities|Casting|CastToBP_PlayerCharacter (Pawn|GetControlledPawn (Variables|Default|GetOwnerController))))
    (Class|IFCharacterPlayer|RecallTurret _asbp_player_character)))

(fn ConstructionScript)