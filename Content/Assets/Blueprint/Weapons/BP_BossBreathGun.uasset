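; BP_BossBreathGun is a boss breath weapon that damages the player with a forward box trace.
; StartBreathTrace plays a timeline from the start, whose track sets the trace length along the actor's forward vector on each update.
; Each update calls GiveDamage if the hit actor is a BP_PlayerCharacter, so damage can repeat while the timeline runs.
; FinishBreathTrace stops the timeline.
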(event EventFinishBreathTrace
  (bind _returnvalue (Transformation|GetActorLocation))
  (bind _newtrack_0 (Timeline|Timeline Stop)
    (:Update
      (bind _output_get (Variables|Default|SetFireLength _newtrack_0))
      (bind _outhit (Collision|BoxTraceByChannel _returnvalue (+ _returnvalue (* (Transformation|GetActorForwardVector) _output_get)) "100.000000,100.000000,70.000000" "0, 0, 0" "TraceTypeQuery7" false 0 "None"))
      (if (Class|GameplayStatics|ObjectIsA (.hitactor _outhit) "/Game/Assets/Blueprint/BP_PlayerCharacter.BP_PlayerCharacter_C")
        (Class|IFGunBase|GiveDamage (.hitactor _outhit))))))

(event EventStartBreathTrace
  (bind _returnvalue (Transformation|GetActorLocation))
  (bind _newtrack_0 (Timeline|Timeline PlayFromStart)
    (:Update
      (bind _output_get (Variables|Default|SetFireLength _newtrack_0))
      (bind _outhit (Collision|BoxTraceByChannel _returnvalue (+ _returnvalue (* (Transformation|GetActorForwardVector) _output_get)) "100.000000,100.000000,70.000000" "0, 0, 0" "TraceTypeQuery7" false 0 "None"))
      (if (Class|GameplayStatics|ObjectIsA (.hitactor _outhit) "/Game/Assets/Blueprint/BP_PlayerCharacter.BP_PlayerCharacter_C")
        (Class|IFGunBase|GiveDamage (.hitactor _outhit))))))

(fn ConstructionScript)