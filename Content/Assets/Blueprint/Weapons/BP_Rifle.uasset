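; BP_Rifle is a rifle weapon Blueprint holding an unfinished hitscan prototype that is not wired to any event, so it never runs.
; The disconnected logic loops ten line traces from the player camera out to MaxRange, ignoring the player character and adding random spread to each endpoint.
; Each trace draws debug lines and prints the hit actor's name, with no damage applied; the construction script is empty.
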(fn ConstructionScript)