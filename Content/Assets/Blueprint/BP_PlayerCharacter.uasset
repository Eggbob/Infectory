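; Player character Blueprint that handles build mode and turret-gadget placement, plus test keys for flight mode and fly speed.
; ACBuildComponent receives the follow camera and drives the Building/Idle state, supplying the placement transform and validity to BuildGadget.
; Turret range is drawn with spline meshes generated from path points, then cleared.
; Flying vertical input uses an up vector derived from actor location, and the audio listener follows the mesh with camera-combined rotation.
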(event Custom|RemoveComponent
  (params (MeshComp :type Actor%20Component%20Object%20Reference))
  (Components|DestroyComponent MeshComp))

(event EventSetAudioLitener
  (bind _returnvalue (Transformation|GetActorRotation))
  (bind _followcamera (Variables|Default|GetFollowCamera))
  (bind _returnvalue_2 (Transformation|GetWorldRotation _followcamera))
  (bind _returnvalue_3 (* _returnvalue -1.0))
  (bind _returnvalue_4 (Math|Conversions|RotationFromXVector _returnvalue_3))
  (bind _returnvalue_5 (Math|Rotator|CombineRotators _returnvalue_4 _returnvalue_2))
  ;[1 1 1] Audio
  (Class|PlayerController|SetAudioListenerOverride (Game|GetPlayerController 0) (Variables|Character|GetMesh) "0, 0, 0" (Math|Rotator|MakeRotator (.roll _returnvalue_5) (.pitch _returnvalue_5) (+ (.yaw _returnvalue_5) 9e+01))))

(event EventBeginPlay
  (Variables|/Game/Assets/Blueprint/Component/AC_BuildComponent.AC_BuildComponent_C|SetCamera (Variables|Default|GetAC_BuildComponent) (Variables|Default|GetFollowCamera)))

(event EventSetBuildMode
  (bind _ac_buildcomponent (Variables|Default|GetAC_BuildComponent))
  (Default|LaunchBuild _ac_buildcomponent)
  (if (Variables|/Game/Assets/Blueprint/Component/AC_BuildComponent.AC_BuildComponent_C|GetbIsBuildingModeOn _ac_buildcomponent)
    (Variables|Default|SetCurCharacterState "Building")
    (else
      (Variables|Default|SetCurCharacterState "Idle"))))

(event EventGetTurretLoc
  (bind _ac_buildcomponent (Variables|Default|GetAC_BuildComponent))
  (Class|IFCharacterPlayer|BuildGadget (.location (Variables|/Game/Assets/Blueprint/Component/AC_BuildComponent.AC_BuildComponent_C|GetBuildTransform _ac_buildcomponent)) (.location (Transformation|GetSocketTransform (Variables|Default|GetTurretSpawn) "Mount" "RTS_World")) (Variables|/Game/Assets/Blueprint/Component/AC_BuildComponent.AC_BuildComponent_C|GetbCanBuild _ac_buildcomponent)))

(event Input|AxisEvents|InputAxisUpDown
  (params (AxisValue :type Float%20%28single-precision%29))
  ;[1 1 1] ForTest
  (if (Utilities|Enum|Equal(Enum) (Variables|/Script/Engine.CharacterMovementComponent|GetMovementMode (Variables|Character|GetCharacterMovement)) "MOVE_Flying")
    (Pawn|Input|AddMovementInput (Math|Vector|GetUpVector (Math|Conversions|RotationFromXVector (Transformation|GetActorLocation))) AxisValue false)))

(event Input|MouseEvents|MouseWheelAxis
  (params (AxisValue :type Float%20%28single-precision%29))
  (if (and (< (Math|Interpolation|FInterpTo (Variables|Default|GetWheelDirection) (+ (/ AxisValue 1e+01) (Variables|Default|GetWheelDirection)) (Utilities|Time|GetWorldDeltaSeconds) 0.0) 1.3) (> (Math|Interpolation|FInterpTo (Variables|Default|GetWheelDirection) (+ (/ AxisValue 1e+01) (Variables|Default|GetWheelDirection)) (Utilities|Time|GetWorldDeltaSeconds) 0.0) -0.9))
    (Variables|Default|SetWheelDirection (Math|Interpolation|FInterpTo (Variables|Default|GetWheelDirection) (+ (/ AxisValue 1e+01) (Variables|Default|GetWheelDirection)) (Utilities|Time|GetWorldDeltaSeconds) 0.0))))

(event Input|KeyboardEvents|G
  (params (Key :type Key%20Structure :default "None"))
  (bind _charactermovement (Variables|Character|GetCharacterMovement))
  ;[1 1 1] ForTest
  (:Pressed
    (|CollapseGraph (Utilities|Enum|Equal(Enum) (Variables|/Script/Engine.CharacterMovementComponent|GetMovementMode _charactermovement) "MOVE_Flying")
      (:else
        (Pawn|Components|CharacterMovement|SetMovementMode (Variables|Character|GetCharacterMovement) "MOVE_Flying" 0))
      (:then
        (Pawn|Components|CharacterMovement|SetMovementMode _charactermovement "MOVE_Walking" 0)))))

(event Input|KeyboardEvents|Q
  (params (Key :type Key%20Structure :default "None"))
  (bind _charactermovement (Variables|Character|GetCharacterMovement))
  ;[1 1 1] ForTest
  (:Pressed
    (Variables|/Script/Engine.CharacterMovementComponent|SetMaxFlySpeed _charactermovement (+ (Variables|/Script/Engine.CharacterMovementComponent|GetMaxFlySpeed _charactermovement) 5e+02))))

(event Input|KeyboardEvents|E
  (params (Key :type Key%20Structure :default "None"))
  (bind _charactermovement (Variables|Character|GetCharacterMovement))
  ;[1 1 1] ForTest
  (:Pressed
    (Variables|/Script/Engine.CharacterMovementComponent|SetMaxFlySpeed _charactermovement (- (Variables|/Script/Engine.CharacterMovementComponent|GetMaxFlySpeed _charactermovement) 5e+02))))

(fn ConstructionScript)

(fn GetTurretLocation
  (return (Transformation|GetSocketTransform (Variables|Default|GetTurretSpawn) "Mount" "RTS_World")))

(fn ShowTurretRange
  (params (PathPosition :type Array%20of%20Vectors))
  (bind _returnvalue (Math|Float|MakeLiteralFloat 0.5))
  (bind _spline (Variables|Default|GetSpline))
  (for (_array_element _array_index) PathPosition
    (Spline|AddSplinePointatIndex _spline _array_element _array_index "World" true))
  (Spline|SetSplinePointType _spline (Utilities|Array|LastIndex PathPosition) "CurveClamped" true)
  (for _index (range 0 (- (Spline|GetNumberOfSplinePoints _spline) 2))
    (bind _returnvalue_2 (AddComponent|AddSplineMeshComponent true))
    (SplineMesh|SetStartScale _returnvalue_2 (Math|Vector2D|MakeVector2D _returnvalue _returnvalue) true :!class /Script/Engine.SplineMeshComponent)
    (SplineMesh|SetEndScale _returnvalue_2 (Math|Vector2D|MakeVector2D _returnvalue _returnvalue) true :!class /Script/Engine.SplineMeshComponent)
    (Utilities|Array|Add (Variables|Default|GetPointArray) _returnvalue_2)
    (SplineMesh|SetStartandEnd _returnvalue_2 (Utilities|Array|Get(acopy) PathPosition _index) (Spline|GetTangentatSplinePoint (Variables|Default|GetSpline) _index "World") (Utilities|Array|Get(acopy) PathPosition (+ _index 1)) (Spline|GetTangentatSplinePoint (Variables|Default|GetSpline) (+ _index 1) "World") true :!class /Script/Engine.SplineMeshComponent)))

(fn DestroyTurretRange
  (bind _pointarray (Variables|Default|GetPointArray))
  (if (> (Utilities|Array|Length _pointarray) 0)
    (Components|DestroyComponent _pointarray)
    (Utilities|Array|Clear (Variables|Default|GetPointArray))
    (Spline|ClearSplinePoints (Variables|Default|GetSpline) true)))

(fn ClearTurretRange
  (for _array_element (Variables|Default|GetPointArray)
    (Components|DestroyComponent _array_element))
  (Utilities|Array|Clear (Variables|Default|GetPointArray))
  (Spline|ClearSplinePoints (Variables|Default|GetSpline) true)
  (Components|DestroyComponent (Variables|/Game/Assets/Blueprint/Component/AC_BuildComponent.AC_BuildComponent_C|GetBuildGhost (Variables|Default|GetAC_BuildComponent))))