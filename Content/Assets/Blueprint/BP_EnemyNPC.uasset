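; BP_EnemyNPC is an enemy character that moves toward a target actor and can lose body parts when hit.
; StartMoving runs AI MoveTo, and PlayGlowEffect sets the mesh materials' Glow parameter.
; PlayHitReaction stops movement, hides the hit bone and plays a sound for head, thigh or other cuts.
; Losing a thigh also calls ChangeNPCMoveMode to switch how the NPC moves.
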(event EventPlayGlowEffect
  (Rendering|Material|SetScalarParameterValueonMaterials (Variables|Character|GetMesh) "Glow" (Variables|Default|GetGlowParam)))

(event EventBeginPlay
  (Collision|IgnoreActorwhenMoving (Variables|Default|GetCapsuleComponent) self true))

(event EventPlayHitReaction
  (params (BoneName :type Name :default "None") (HitResult :type Hit%20Result%20Structure))
  (Components|Movement|StopMovementImmediately (Variables|Character|GetCharacterMovement))
  (if (Utilities|Set|Contains (Variables|Default|GetBoneName) BoneName)
    (Components|SkinnedMesh|HideBonebyName (Variables|Character|GetMesh) BoneName "PBO_None")
    (if (or (== BoneName (Variables|Default|GetLeftThigh)) (== BoneName (Variables|Default|GetRightThigh)))
      (Audio|PlaySoundatLocation "/Game/Assets/Sound/Monster/monster_hit/SC_EnemyFall.SC_EnemyFall" "0, 0, 0" "0, 0, 0" 1.0 1.0 0.0 0 0 0 0)
      (Class|IFCharacterNonPlayer|ChangeNPCMoveMode)
      (elif (== BoneName (Variables|Default|GetHead))
        (Audio|PlaySoundatLocation "/Game/Assets/Sound/Monster/monster_hit/SC_EnemyHeadCut.SC_EnemyHeadCut" "0, 0, 0" "0, 0, 0" 1.0 1.0 0.0 0 0 0 0)
        (else
          (Audio|PlaySoundatLocation "/Game/Assets/Sound/Monster/monster_hit/SC_EnemyCut.SC_EnemyCut" "0, 0, 0" "0, 0, 0" 1.0 1.0 0.0 0 0 0 0))))))

(event EventStartMoving
  (AI|AIMoveTo self "0, 0, 0" (Variables|Default|GetTargetActor) 5.0 false))

(fn ConstructionScript)