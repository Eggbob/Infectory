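; Player character component that runs a toggleable build mode, previewing placement with a cube ghost; actual building is not handled here.
; BuildCycle re-runs on a short delay, predicting a projectile arc from the turret, scaled by WheelDirection, to position the ghost.
; A box trace at the landing point sets CanBuild and the ghost's green or red material.
; The arc display is cleared every Tick; CalcDirection's ballistic math is unused here.
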(event Custom|BuildDelay
  (if (Variables|Default|GetbIsBuildingModeOn)
    (Utilities|FlowControl|Delay 0.01)
    (CallFunction|BuildCycle)
    (else
      (Variables|Default|SetbIsBuildingModeOn false)
      (Variables|Default|SetbCanBuild false)
      (Default|RemoveComponent (Variables|Default|GetPlayerReference) (Variables|Default|GetBuildGhost)))))

(event Custom|LaunchBuild
  (if (Variables|Default|GetbIsBuildingModeOn)
    (CallFunction|StopBuildMode)
    (else
      (Variables|Default|SetbIsBuildingModeOn true)
      (CallFunction|BuildCycle)))
  (Default|DestroyTurretRange (Variables|Default|GetPlayerReference)))

(event Custom|StopBuildMode
  (Variables|Default|SetbIsBuildingModeOn false)
  (Variables|Default|SetbCanBuild false)
  (Default|RemoveComponent (Variables|Default|GetPlayerReference) (Variables|Default|GetBuildGhost)))

(event EventBeginPlay
  (bind _asbp_player_character (Utilities|Casting|CastToBP_PlayerCharacter (Components|GetOwner)))
  (Variables|Default|SetPlayerReference _asbp_player_character))

(event EventTick
  (params (DeltaSeconds :type Float%20%28single-precision%29))
  (Default|DestroyTurretRange (Variables|Default|GetPlayerReference)))

(fn SpawnBuildGhost
  (Utilities|IsValid (Variables|Default|GetBuildGhost)
    (:Is%20Valid
      (Development|SetHiddeninGame (Variables|Default|GetBuildGhost) false false))
    (:Is%20Not%20Valid
      (bind _returnvalue (Game|AddComponentbyClass (Variables|Default|GetPlayerReference) "/Script/Engine.StaticMeshComponent" true (Variables|Default|GetBuildTransform)))
      (bind _output_get (Variables|Default|SetBuildGhost _returnvalue))
      (Components|StaticMesh|SetStaticMesh _output_get "/Engine/BasicShapes/Cube.Cube")
      (Collision|SetCollisionEnabled (Variables|Default|GetBuildGhost) "NoCollision"))))

(fn GiveBuildColor
  (params (bIsGreen :type Boolean))
  (Variables|Default|SetbCanBuild bIsGreen)
  (for _index (range (- (Rendering|Material|GetNumMaterials (Variables|Default|GetBuildGhost)) 1) 0)
    (if bIsGreen
      (Rendering|Material|SetMaterial (Variables|Default|GetBuildGhost) _index "/Game/Assets/Art/M_GreeColor.M_GreeColor")
      (else
        (Rendering|Material|SetMaterial (Variables|Default|GetBuildGhost) _index "/Game/Assets/Art/M_RedColor.M_RedColor"))))
  (Transformation|SetWorldTransform (Variables|Default|GetBuildGhost) (Variables|Default|GetBuildTransform) false false))

(fn BuildCycle
  (bind _buildghost (Variables|Default|GetBuildGhost))
  (bind _returnvalue (Rendering|IsVisible _buildghost))
  (bind _returnvalue_2 (Default|GetTurretLocation (Variables|Default|GetPlayerReference)))
  (bind (_outhit _outpathpositions _outlasttracedestination _returnvalue_3) (Class|GameplayStatics|BlueprintPredictProjectilePathbyTraceChannel (.location _returnvalue_2) (* (+ (Math|Vector|GetForwardVector (.rotation _returnvalue_2)) (* (Math|Vector|GetForwardVector (.rotation _returnvalue_2)) (Variables|/Game/Assets/Blueprint/BP_PlayerCharacter.BP_PlayerCharacter_C|GetWheelDirection (Variables|Default|GetPlayerReference)))) 1000) true 2e+01 "ECC_GameTraceChannel7" false 0 "None" 0.0 12.0 1e+01))
  (Default|ShowTurretRange (Variables|Default|GetPlayerReference) _outpathpositions)
  (if _returnvalue_3
    (bind _returnvalue_4 (Collision|BoxTraceByChannel (+ (.Location (Collision|BreakHitResult _outhit)) "0.000000,0.000000,70.000000") (+ (.Location (Collision|BreakHitResult _outhit)) "0.000000,0.000000,40.000000") "45.000000,45.000000,30.000000" "0, 0, 0" "TraceTypeQuery5" false 0 "None" true "(R=0.000000,G=0.210779,B=1.000000,A=1.000000)"))
    (Variables|Default|SetBuildTransform (Math|Transform|MakeTransform (.Location (Collision|BreakHitResult _outhit)) (.rotation (Variables|Default|GetBuildTransform)) (.scale (Variables|Default|GetBuildTransform))))
    (Utilities|IsValid _buildghost
      (:Is%20Valid
        (if _returnvalue
          (if _returnvalue_4
            (CallFunction|GiveBuildColor false)
            (else
              (CallFunction|GiveBuildColor true)))
          (else
            (CallFunction|SpawnBuildGhost :!label _label))))
      (:Is%20Not%20Valid
        (goto _label)))
    (else
      (bind _returnvalue_5 (Collision|BoxTraceByChannel (.TraceEnd (Collision|BreakHitResult _outhit)) (- (.TraceEnd (Collision|BreakHitResult _outhit)) "0.000000,0.000000,70.000000") "45.000000,45.000000,30.000000" "0, 0, 0" "TraceTypeQuery5" false 0 "None" true "(R=0.000000,G=0.210779,B=1.000000,A=1.000000)"))
      (Variables|Default|SetBuildTransform (Math|Transform|MakeTransform (.Location (Collision|BreakHitResult _outhit)) (.rotation (Variables|Default|GetBuildTransform)) (.scale (Variables|Default|GetBuildTransform))))
      (Utilities|IsValid _buildghost
        (:Is%20Valid
          (if _returnvalue
            (if _returnvalue_5
              (CallFunction|GiveBuildColor false)
              (else
                (CallFunction|GiveBuildColor true)))
            (else
              (goto _label))))
        (:Is%20Not%20Valid
          (goto _label)))))
  (CallFunction|BuildDelay))

(fn CalcDirection
  (bind _camera (Variables|Default|GetCamera))
  (bind _buildtransform (Variables|Default|GetBuildTransform))
  (bind _returnvalue (Transformation|GetWorldLocation _camera))
  (bind _returnvalue_2 (- (.location _buildtransform) _returnvalue))
  (bind _output_get (Variables|Default|SetLaunchDirec (Math|Vector|MakeVector (.x _returnvalue_2) (.y _returnvalue_2) 0.0)))
  (bind _output_get_2 (Variables|Default|SetTimeToTarget (/ (Math|Vector|VectorLength _output_get) (Variables|Default|GetProjectileSpeed))))
  (bind _output_get_3 (Variables|Default|SetLaunchVelocity (Math|Vector|MakeVector (.x (/ (Variables|Default|GetLaunchDirec) _output_get_2)) (.y (/ (Variables|Default|GetLaunchDirec) _output_get_2)) (+ (.z (/ (Variables|Default|GetLaunchDirec) _output_get_2)) (* (* (Variables|Default|GetGravity) (Variables|Default|GetTimeToTarget)) 0.5)))))
  (Default|GetTurretLocation (Variables|Default|GetPlayerReference)))