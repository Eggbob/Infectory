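; Trigger-driven map wall that closes when its Box is overlapped and is removed when a second box is overlapped.
; Box destroys itself, plays audio and runs a timeline that moves SciFiWalls.
; Delays chained off the timeline's Update spawn asphalt particles at two billboards, remove them, then light a SpotLight hidden since BeginPlay with more audio.
; Overlapping Wall_open_box destroys the wall and spotlight outright.
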(event OnComponentBeginOverlap(Box)
  (params (OverlappedComponent :type Primitive%20Component%20Object%20Reference) (OtherActor :type Actor%20Object%20Reference) (OtherComp :type Primitive%20Component%20Object%20Reference) (OtherBodyIndex :type Integer) (bFromSweep :type Boolean) (SweepResult :type Hit%20Result%20Structure%20%28by%20ref%29))
  (bind _billboard (Variables|Default|GetBillboard))
  (bind _spotlight (Variables|Default|GetSpotLight))
  (AddComponent|AddAudioComponent false)
  (Components|DestroyComponent (Variables|Default|GetBox))
  (bind _새_트랙_1 (Timeline|내려감 Play)
    (:Update
      (Transformation|SetRelativeLocation (Variables|Default|Getsci_fi_walls) _새_트랙_1 false false)
      (Utilities|FlowControl|Delay 2.0)
      (Effects|SpawnEmitteratLocation "/Game/Realistic_Starter_VFX_Pack_Vol2/Particles/Hit/P_Asphalt.P_Asphalt" (Transformation|GetWorldLocation (Variables|Default|GetBillboard)))
      (Effects|SpawnEmitteratLocation "/Game/Realistic_Starter_VFX_Pack_Vol2/Particles/Hit/P_Asphalt.P_Asphalt" (Transformation|GetWorldLocation (Variables|Default|GetBillboard1)))
      (Components|Activation|Deactivate _billboard)
      (Rendering|SetVisibility (Variables|Default|GetBillboard) false false)
      (Components|DestroyComponent _billboard)
      (Utilities|FlowControl|Delay 0.6)
      (Rendering|SetVisibility _spotlight true false)
      (Components|Activation|Activate _spotlight false)
      (AddComponent|AddAudioComponent false))))

(event OnComponentBeginOverlap(Wall_open_box)
  (params (OverlappedComponent :type Primitive%20Component%20Object%20Reference) (OtherActor :type Actor%20Object%20Reference) (OtherComp :type Primitive%20Component%20Object%20Reference) (OtherBodyIndex :type Integer) (bFromSweep :type Boolean) (SweepResult :type Hit%20Result%20Structure%20%28by%20ref%29))
  (Components|DestroyComponent (Variables|Default|GetSpotLight)))

(event EventBeginPlay
  (bind _spotlight (Variables|Default|GetSpotLight))
  (Rendering|SetVisibility _spotlight false false)
  (Components|Activation|Deactivate _spotlight))

(fn ConstructionScript)