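; BP_04_Laptop is an interactable map laptop that switches from a red state to a blue one when the player presses E nearby.
; A box overlap enables and disables input on the actor for player controller 0.
; BeginPlay hides and deactivates LaptopBlue; pressing E prints a debug string, hides and deactivates LaptopRed, then shows and activates LaptopBlue, with no path back.
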(event OnComponentEndOverlap(Box)
  (params (OverlappedComponent :type Primitive%20Component%20Object%20Reference) (OtherActor :type Actor%20Object%20Reference) (OtherComp :type Primitive%20Component%20Object%20Reference) (OtherBodyIndex :type Integer))
  (Input|DisableInput (Game|GetPlayerController 0)))

(event OnComponentBeginOverlap(Box)
  (params (OverlappedComponent :type Primitive%20Component%20Object%20Reference) (OtherActor :type Actor%20Object%20Reference) (OtherComp :type Primitive%20Component%20Object%20Reference) (OtherBodyIndex :type Integer) (bFromSweep :type Boolean) (SweepResult :type Hit%20Result%20Structure%20%28by%20ref%29))
  (Input|EnableInput (Game|GetPlayerController 0)))

(event EventBeginPlay
  (bind _laptop_blue (Variables|Default|Getlaptop_blue))
  (Rendering|SetVisibility _laptop_blue false false)
  (Components|Activation|Deactivate _laptop_blue))

(event Input|KeyboardEvents|E
  (params (Key :type Key%20Structure))
  (bind _laptop_blue (Variables|Default|Getlaptop_blue))
  (bind _laptop_red (Variables|Default|Getlaptop_red))
  (:Pressed
    (Development|PrintString "시팔")
    (Rendering|SetVisibility _laptop_red false false)
    (Components|Activation|Deactivate _laptop_red)
    (Rendering|SetVisibility _laptop_blue true false)
    (Components|Activation|Activate _laptop_blue false)))

(event Input|KeyboardEvents|E
  (params (Key :type Key%20Structure)))

(fn ConstructionScript)