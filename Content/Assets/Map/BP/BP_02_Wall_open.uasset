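; Interactive wall-opening Blueprint that fires a one-time explosion and lighting change when E is pressed inside its Box trigger.
; Box overlap enables and disables the actor's input, and the mint and white lights start hidden.
; E adds audio, destroys the Box, spawns an explosion at the Billboard and hides it, then swaps the orange lights for the mint and white ones.
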(event OnComponentEndOverlap(Box)
  (params (OverlappedComponent :type Primitive%20Component%20Object%20Reference) (OtherActor :type Actor%20Object%20Reference) (OtherComp :type Primitive%20Component%20Object%20Reference) (OtherBodyIndex :type Integer))
  ;[1 1 1] E를 누르는 영역 지정
  (Input|DisableInput (Game|GetPlayerController 0)))

(event OnComponentBeginOverlap(Box)
  (params (OverlappedComponent :type Primitive%20Component%20Object%20Reference) (OtherActor :type Actor%20Object%20Reference) (OtherComp :type Primitive%20Component%20Object%20Reference) (OtherBodyIndex :type Integer) (bFromSweep :type Boolean) (SweepResult :type Hit%20Result%20Structure%20%28by%20ref%29))
  ;[1 1 1] E를 누르는 영역 지정
  (Input|EnableInput (Game|GetPlayerController 0)))

(event EventBeginPlay
  (bind _pointlight_mint (Variables|Default|GetPointLight_mint))
  (Rendering|SetVisibility _pointlight_mint false false)
  (Components|Activation|Deactivate _pointlight_mint))

(event Input|KeyboardEvents|E
  (params (Key :type Key%20Structure :default "None"))
  (bind _pointlight_orange (Variables|Default|GetPointLight_Orange))
  (bind _pointlight_mint (Variables|Default|GetPointLight_mint))
  (:Pressed
    (AddComponent|AddAudioComponent false)
    (Components|DestroyComponent (Variables|Default|GetBox))
    (Effects|SpawnEmitteratLocation "/Game/Realistic_Starter_VFX_Pack_Vol2/Particles/Explosion/P_Explosion_Big_A.P_Explosion_Big_A" (Transformation|GetWorldLocation (Variables|Default|GetBillboard)))
    (Rendering|SetVisibility _pointlight_orange false false)
    (Components|Activation|Deactivate _pointlight_orange)
    (Rendering|SetVisibility _pointlight_mint true false)
    (Components|Activation|Activate _pointlight_mint false)))

(fn ConstructionScript)