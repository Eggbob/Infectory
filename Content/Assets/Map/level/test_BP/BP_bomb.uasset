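; BP_bomb is an explosive barrel that detonates when something overlaps its blast-range component (폭발범위).
; If the barrel flag set at BeginPlay is true, it spawns a scaled-up Molotov particle effect and destroys the barrel and range components.
; It then calls ApplyDamage with environmental damage but no target connected, and ends by assigning 폭발딜링범위 to itself.
; The flag is never cleared.
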(event OnComponentBeginOverlap(폭발범위)
  (params (OverlappedComponent :type Primitive%20Component%20Object%20Reference) (OtherActor :type Actor%20Object%20Reference) (OtherComp :type Primitive%20Component%20Object%20Reference) (OtherBodyIndex :type Integer) (bFromSweep :type Boolean) (SweepResult :type Hit%20Result%20Structure%20%28by%20ref%29))
  (if (Variables|Default|Get폭발통이%20있나?)
    (Effects|SpawnEmitteratLocation "/Game/Realistic_Starter_VFX_Pack_Vol2/Particles/Explosion/P_Molotov.P_Molotov" (Transformation|GetWorldLocation (Variables|Default|Get폭발)) "0, 0, 0" "6.000000,6.000000,6.000000")
    (Components|DestroyComponent (Variables|Default|Get폭발통))
    (Game|Damage|ApplyDamage 0 55.0 0 0 "/Engine/EngineDamageTypes/DmgTypeBP_Environmental.DmgTypeBP_Environmental_C")
    (Variables|Default|Set폭발%20딜링%20범위 (Variables|Default|Get폭발%20딜링%20범위))))

(event Collision|EventActorBeginOverlap
  (params (OtherActor :type Actor%20Object%20Reference)))

(event EventTick
  (params (DeltaSeconds :type Float%20%28single-precision%29)))

(event EventBeginPlay
  (Variables|Default|Set폭발통이%20있나? true))

(fn ConstructionScript)