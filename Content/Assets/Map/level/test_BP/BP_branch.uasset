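; Test level Blueprint for a breakable wall that explodes when something overlaps its trigger, 도착지점 (arrival point).
; BeginPlay clears the 플레이어발판 (player pad) flag; any overlap sets it, without filtering the actor, and calls 벽부수는조건 (wall-break condition).
; That event brightens the light, spawns an attached explosion, destroys the wall and trigger, and plays a world camera shake.
; Its light-off branch is never reached through this overlap path.
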(event OnComponentBeginOverlap(도착지점)
  (params (OverlappedComponent :type Primitive%20Component%20Object%20Reference) (OtherActor :type Actor%20Object%20Reference) (OtherComp :type Primitive%20Component%20Object%20Reference) (OtherBodyIndex :type Integer) (bFromSweep :type Boolean) (SweepResult :type Hit%20Result%20Structure%20%28by%20ref%29))
  (Variables|Default|Set플레이어%20발판 true)
  (CallFunction|벽부수는조건))

(event Custom|벽%20부수는%20조건
  (if (Variables|Default|Get플레이어%20발판)
    (Rendering|Components|Light|SetIntensity (Variables|Default|Get조명) 1.5e+04)
    (Effects|SpawnEmitterAttached "/Game/Realistic_Starter_VFX_Pack_Vol2/Particles/Explosion/P_Explosion_Big_B.P_Explosion_Big_B" (Variables|Default|Get폭발) "None" "119.384429,0.539431,195.400982" "0, 0, 0" "4.000000,4.000000,4.000000")
    (Components|DestroyComponent (Variables|Default|Get벽))
    (Collision|SetCollisionEnabled (Variables|Default|Get벽) "NoCollision")
    (Camera|PlayWorldCameraShake "/Script/GameplayCameras.DefaultCameraShakeBase" "455.496012,544.125906,0.000029" 1e+02 1e+02 1e+01 true)
    (else
      (Rendering|Components|Light|SetIntensity (Variables|Default|Get조명) 0.0))))

(event EventBeginPlay
  (Variables|Default|Set플레이어%20발판 false))

(fn ConstructionScript)