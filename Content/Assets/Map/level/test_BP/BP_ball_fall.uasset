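; Falling monster ball actor, apparently a test map hazard, that drops once when triggered by overlap.
; An overlap on BallFallingCollision arms it through AttachToCeiling, and an actor overlap while armed sets IsStart, hides that collision component, adds audio and calls PlayBall.
; The BallFalling timeline drives MonsterBall's relative location without sweep, then spawns a poison impact particle and destroys the ball component.
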(event OnComponentBeginOverlap(BallShooterCollision)
  (params (OverlappedComponent :type Primitive%20Component%20Object%20Reference) (OtherActor :type Actor%20Object%20Reference) (OtherComp :type Primitive%20Component%20Object%20Reference) (OtherBodyIndex :type Integer) (bFromSweep :type Boolean) (SweepResult :type Hit%20Result%20Structure%20%28by%20ref%29)))

(event OnComponentBeginOverlap(BallFallingCollision)
  (params (OverlappedComponent :type Primitive%20Component%20Object%20Reference) (OtherActor :type Actor%20Object%20Reference) (OtherComp :type Primitive%20Component%20Object%20Reference) (OtherBodyIndex :type Integer) (bFromSweep :type Boolean) (SweepResult :type Hit%20Result%20Structure%20%28by%20ref%29))
  (if (not (Variables|Default|GetbIsStart))
    (Variables|Default|SetbAttachToCeiling true)))

(event Custom|PlayBall
  (bind _fallingloop (Timeline|BallFalling Play)
    (:Update
      (Transformation|SetRelativeLocation (Variables|Default|GetMonsterBall) _fallingloop false false))
    (:Finished
      (Effects|SpawnEmitteratLocation "/Game/InfinityBladeEffects/Effects/FX_Skill_Leap/P_Skill_Leap_Poison_Velocity_Impact.P_Skill_Leap_Poison_Velocity_Impact" (Transformation|GetWorldLocation (Variables|Default|GetMonsterBall)) "0, 0, 0" "1.000000,1.000000,1.000000" true "AutoRelease")
      (Components|DestroyComponent (Variables|Default|GetMonsterBall)))))

(event Collision|EventActorBeginOverlap
  (params (OtherActor :type Actor%20Object%20Reference))
  (if (and (Variables|Default|GetbAttachToCeiling) (not (Variables|Default|GetbIsStart)))
    (Variables|Default|SetbIsStart true)
    (Development|SetHiddeninGame (Variables|Default|GetBallFallingCollision) true false)
    (AddComponent|AddAudioComponent false)
    (CallFunction|PlayBall)))

(event EventBeginPlay
  (Variables|Default|SetbAttachToCeiling false))

(fn ConstructionScript)