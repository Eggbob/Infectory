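; Large two-panel map door that moves when a player presses E near it.
; Box overlap enables or disables input from player 0 on this actor, without checking which actor overlaps.
; E plays timelines that set DoorUp and DoorDown relative locations, then after a delay a second pair moves both again.
; Each timeline chains from the previous one's Update pin, and all use Play rather than PlayFromStart, with no reset.
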(event OnComponentBeginOverlap(Box)
  (params (OverlappedComponent :type Primitive%20Component%20Object%20Reference) (OtherActor :type Actor%20Object%20Reference) (OtherComp :type Primitive%20Component%20Object%20Reference) (OtherBodyIndex :type Integer) (bFromSweep :type Boolean) (SweepResult :type Hit%20Result%20Structure%20%28by%20ref%29))
  (Input|EnableInput (Game|GetPlayerController 0)))

(event OnComponentEndOverlap(Box)
  (params (OverlappedComponent :type Primitive%20Component%20Object%20Reference) (OtherActor :type Actor%20Object%20Reference) (OtherComp :type Primitive%20Component%20Object%20Reference) (OtherBodyIndex :type Integer))
  (Input|DisableInput (Game|GetPlayerController 0)))

(event Input|KeyboardEvents|E
  (params (Key :type Key%20Structure :default "None"))
  (:Pressed
    (bind _새_트랙_0 (Timeline|타임라인 Play)
      (:Update
        (Transformation|SetRelativeLocation (Variables|Default|Getdoor_up) _새_트랙_0 false false)
        (bind _새_트랙_0_2 (Timeline|타임라인_0 Play)
          (:Update
            (Transformation|SetRelativeLocation (Variables|Default|Getdoor_down) _새_트랙_0_2 false false)
            (Utilities|FlowControl|Delay 3.0)
            (bind _새_트랙_0_3 (Timeline|타임라인_1 Play)
              (:Update
                (Transformation|SetRelativeLocation (Variables|Default|Getdoor_up) _새_트랙_0_3 false false)
                (bind _새_트랙_0_4 (Timeline|타임라인_2 Play)
                  (:Update
                    (Transformation|SetRelativeLocation (Variables|Default|Getdoor_down) _새_트랙_0_4 false false)))))))))))

(fn ConstructionScript)